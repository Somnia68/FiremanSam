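; BurnableEntitiesManager is a component that keeps a registry of burnable entities and spreads their updates across frames.
; Add and remove events maintain the array and its count, and ticking starts after a short delay following BeginPlay.
; Each tick calls update on a rolling slice sized by the tick rate, wrapping to the start at the end.
; Delta time is scaled by the count-to-rate ratio, inverted for wrapped entries.
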(event Custom|Ready
  (Components|Tick|SetComponentTickEnabled true))

(event Custom|AddBurnableEntity
  (params (NewItem :type Burnt%20Base%20Object%20Reference%20%28by%20ref%29))
  (Utilities|Array|Add (Variables|Default|GetBurnableEntityArray) NewItem)
  (Math|Integer|IncrementInt (Variables|Default|GetPipelineTotal)))

(event Custom|RemoveBurnableEntity
  (params (Item :type Burnt%20Base%20Object%20Reference%20%28by%20ref%29))
  (bind _burnableentityarray (Variables|Default|GetBurnableEntityArray))
  (Utilities|Array|RemoveItem _burnableentityarray Item)
  (bind _result (Math|Integer|DecrementInt (Variables|Default|GetPipelineTotal))
    (:%20%20
      (Utilities|Array|Resize _burnableentityarray _result))))

(event EventBeginPlay
  (Components|Tick|SetComponentTickEnabled false)
  (Utilities|FlowControl|Delay 2.0)
  (CallFunction|Ready))

(event EventTick
  (params (DeltaSeconds :type Float%20%28single-precision%29))
  (bind _pipelinetickrate (Variables|Default|GetPipelineTickRate))
  (bind _pipelinetotal (Variables|Default|GetPipelineTotal))
  (Variables|Default|SetPipelineTickIndex 0)
  (for _index (range (Variables|Default|GetPipelineIndex) (Math|Integer|Clamp(Integer) (+ (Variables|Default|GetPipelineIndex) (- (Variables|Default|GetPipelineTickRate) 1)) 0 _pipelinetotal))
    (Math|Integer|IncrementInt (Variables|Default|GetPipelineTickIndex)
      (:%20%20
        (Default|CallUpdateEntity (Utilities|Array|Get(acopy) (Variables|Default|GetBurnableEntityArray) _index) (* DeltaSeconds (/ (Math|Conversions|ToFloat(Integer) (Variables|Default|GetPipelineTotal)) (Math|Conversions|ToFloat(Integer) (Variables|Default|GetPipelineTickRate))))))))
  (if (>= (+ (Variables|Default|GetPipelineIndex) (- (Variables|Default|GetPipelineTickRate) 1)) _pipelinetotal)
    (Variables|Default|SetPipelineIndex 0)
    (for _index_2 (range 0 (Math|Integer|Clamp(Integer) (- _pipelinetickrate (+ (Variables|Default|GetPipelineTickIndex) 1)) 0 _pipelinetickrate))
      (Math|Integer|IncrementInt (Variables|Default|GetPipelineTickIndex)
        (:%20%20
          (Default|CallUpdateEntity (Utilities|Array|Get(acopy) (Variables|Default|GetBurnableEntityArray) _index_2) (* DeltaSeconds (/ (Math|Conversions|ToFloat(Integer) (Variables|Default|GetPipelineTickRate)) (Math|Conversions|ToFloat(Integer) (Variables|Default|GetPipelineTotal))))))))
    (bind _output_get (Variables|Default|SetPipelineIndex (Math|Integer|Clamp(Integer) (- _pipelinetickrate (+ (Variables|Default|GetPipelineTickIndex) 1)) 0 _pipelinetickrate)))
    (Math|Integer|IncrementInt _output_get)
    (else
      (bind _output_get_2 (Variables|Default|SetPipelineIndex (Math|Integer|Clamp(Integer) (+ (Variables|Default|GetPipelineIndex) (- (Variables|Default|GetPipelineTickRate) 1)) 0 _pipelinetotal)))
      (Math|Integer|IncrementInt _output_get_2))))