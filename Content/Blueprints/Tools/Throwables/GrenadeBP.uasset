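; GrenadeBP is a thrown grenade that applies water to nearby Burnt_Base actors on impact.
; BeginPlay launches the physics mesh with GrenadeVelocity.
; The first hit hides the mesh, activates the particle system and runs a wide, flat capsule trace over world static and dynamic objects.
; Each Burnt_Base hit receives Water with the grenade's Power, and the actor destroys itself after a short delay.
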(event OnComponentHit(GrenadeMesh)
  (params (HitComponent :type Primitive%20Component%20Object%20Reference) (OtherActor :type Actor%20Object%20Reference) (OtherComp :type Primitive%20Component%20Object%20Reference) (NormalImpulse :type Vector :default "0, 0, 0") (Hit :type Hit%20Result%20Structure%20%28by%20ref%29))
  (bind _grenademesh (Variables|Default|GetGrenadeMesh))
  (bind _returnvalue (Transformation|GetWorldLocation _grenademesh))
  (if (not (Variables|Default|GetActivated))
    (Rendering|SetVisibility (Variables|Default|GetGrenadeMesh) false false)
    (Components|Activation|Activate (Variables|Default|GetParticleSystem) false)
    (Variables|Default|SetActivated true)
    (bind _outhits (Class|KismetSystemLibrary|CapsuleTraceMultiforObjects (+ _returnvalue "0, 0,-10.000000") (+ _returnvalue "0, 0,10.000000") 4e+02 2.0 (Utilities|Array|MakeArray "ObjectTypeQuery2" "ObjectTypeQuery1") false 0 "None" true "(R=1.000000,G=0.000000,B=0.000000,A=1.000000)" "(R=0.000000,G=1.000000,B=0.000000,A=1.000000)" 3.0))
    (for _array_element _outhits
      (bind _asburnt_base (Utilities|Casting|CastToBurnt_Base (.HitActor (Collision|BreakHitResult _array_element))))
      (Default|Water _asburnt_base (Variables|Default|GetPower)))
    (Utilities|FlowControl|Delay 4.0)
    (Actor|DestroyActor)))

(event EventBeginPlay
  (Physics|SetPhysicsLinearVelocity (Variables|Default|GetGrenadeMesh) (Variables|Default|GetGrenadeVelocity) false "None"))

(fn ConstructionScript)