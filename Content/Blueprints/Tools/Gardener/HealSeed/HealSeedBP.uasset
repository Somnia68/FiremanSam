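; HealSeedBP is a gardener tool actor that gives a one-time health boost to nearby trees.
; One second after BeginPlay, it runs a wide, flat capsule multi-trace for WorldDynamic objects around itself, with debug drawing on.
; Each TreeEntityActorBP hit that is not smoking gains health scaled by its Degrade value, clamped to a fixed range.
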(event EventBeginPlay
  (bind _returnvalue (Transformation|GetActorLocation))
  (Utilities|FlowControl|Delay 1.0)
  (bind _outhits (Class|KismetSystemLibrary|CapsuleTraceMultiforObjects (+ _returnvalue "0, 0,-10.000000") (+ _returnvalue "0, 0,10.000000") 4e+02 2.0 (Utilities|Array|MakeArray "ObjectTypeQuery2") false 0 "ForOneFrame" true "(R=0.813974,G=1.000000,B=0.000000,A=1.000000)" "(R=0.000000,G=1.000000,B=0.000000,A=1.000000)" 3.0))
  (for _array_element _outhits
    (bind _astree_entity_actor_bp (Utilities|Casting|CastToTreeEntityActorBP (.HitActor (Collision|BreakHitResult _array_element))))
    (if (not (Variables|/Game/Blueprints/Nature/Trees/TreeEntityActorBP.TreeEntityActorBP_C|GetisSmoking _astree_entity_actor_bp))
      (Variables|/Game/Blueprints/Nature/Trees/TreeEntityActorBP.TreeEntityActorBP_C|SetHealth _astree_entity_actor_bp (Math|Float|Clamp(Float) (+ (Variables|/Game/Blueprints/Nature/Trees/TreeEntityActorBP.TreeEntityActorBP_C|GetHealth _astree_entity_actor_bp) (* (Variables|/Game/Blueprints/Nature/Trees/TreeEntityActorBP.TreeEntityActorBP_C|GetDegrade _astree_entity_actor_bp) 1e+01)) 0.0 4e+02)))))

(event Collision|EventActorBeginOverlap
  (params (OtherActor :type Actor%20Object%20Reference)))

(event EventTick
  (params (DeltaSeconds :type Float%20%28single-precision%29)))

(fn ConstructionScript)