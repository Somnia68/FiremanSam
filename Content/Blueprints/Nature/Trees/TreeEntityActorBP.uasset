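; Tree actor that simulates heat, smoke, fire spread and burning, and registers with the gamemode's TreeManagerComponent.
; UpdateEvent integrates heat from accumulated rates and toggles smoke and fire at thresholds; smoking feeds its own heat, while Water cools it.
; A burning tree loses health until it swaps to a burnt mesh, and adds heat rate to neighbours cached by a capsule trace at setup.
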(event Custom|UpdateEvent
  (params (Delta :type Float%20%28single-precision%29))
  (bind _isburnt (Variables|Fire|GetisBurnt))
  (bind _isonfire (Variables|Fire|GetisOnFire))
  (bind _issmoking (Variables|Smoke|GetisSmoking))
  (Variables|Heat|SetHeatCurrent (Math|Float|Clamp(Float) (+ (Variables|Heat|GetHeatCurrent) (* Delta (Variables|Heat|GetHeatRateTotal))) 0.0 (Variables|Heat|GetHeatMax)))
  (Utilities|FlowControl|Sequence
    (:then_0
      (if (>= (Variables|Heat|GetHeatCurrent) (Variables|Heat|GetHeatSmoke))
        (if (not _issmoking)
          (CallFunction|StartSmoke))
        (elif _issmoking
          (CallFunction|EndSmoke))))
    (:then_1
      (if (>= (Variables|Heat|GetHeatCurrent) (Variables|Heat|GetHeatFire))
        (if (not _isonfire)
          (CallFunction|StartFire))
        (elif _isonfire
          (CallFunction|EndFire))))
    (:then_2
      (if (Variables|Fire|GetisOnFire)
        (bind _output_get (Variables|Fire|SetHealth (- (Variables|Fire|GetHealth) (* (Variables|Fire|GetDegrade) Delta)))))
      (if (<= _output_get (Variables|Fire|GetBurntState))
        (if (not _isburnt)
          (CallFunction|SetBurnt))
        (elif _isburnt
          (CallFunction|SetRegrown))))))

(event Custom|AddHeatRate
  (params (BurnRate :type Float%20%28single-precision%29))
  (Variables|Heat|SetHeatRateTotal (+ BurnRate (Variables|Heat|GetHeatRateTotal))))

(event Custom|TreeBurnt
  (CallFunction|SetBurnt))

(event Custom|Setup
  (Utilities|FlowControl|Sequence
    (:then_0
      (CallFunction|StopAllParticles)
      (CallFunction|GetNearbyTrees)
      (Variables|Fire|SetHealth 4e+02)
      (Variables|Heat|SetHeatCurrent 0.0))
    (:then_1
      (Variables|GameState|SetisReady true)
      (CallFunction|UpdateEvent 0.0))))

(event Custom|Water
  (params (Rate :type Float%20%28single-precision%29))
  (Variables|Heat|SetHeatCurrent (Math|Float|Clamp(Float) (- (Variables|Heat|GetHeatCurrent) Rate) 0.0 1e+02)))

(event Custom|StartSmoke
  (Variables|Smoke|SetisSmoking true)
  (CallFunction|UpdateSmokeSystem true)
  (CallFunction|AddHeatRate (Variables|Heat|GetHeatRateSelf)))

(event Custom|TreeGrown
  (CallFunction|SetRegrown))

(event Custom|EndSmoke
  (Variables|Smoke|SetisSmoking false)
  (CallFunction|UpdateSmokeSystem false)
  (CallFunction|SubtractHeatRate (Variables|Heat|GetHeatRateSelf)))

(event Custom|SubtractHeatRate
  (params (BurnRate :type Float%20%28single-precision%29))
  (Variables|Heat|SetHeatRateTotal (Math|Float|Clamp(Float) (- (Variables|Heat|GetHeatRateTotal) BurnRate) 0.0 (Variables|Heat|GetHeatMax))))

(event Custom|StartFire
  (Variables|Fire|SetisOnFire true)
  (CallFunction|UpdateFireSystem true)
  (for _array_element (Variables|Default|GetNearby)
    (CallFunction|AddHeatRate _array_element (Variables|Heat|GetHeatRateSelf))))

(event Custom|EndFire
  (Variables|Fire|SetisOnFire false)
  (CallFunction|UpdateFireSystem false)
  (for _array_element (Variables|Default|GetNearby)
    (CallFunction|SubtractHeatRate _array_element (Variables|Heat|GetHeatRateSelf))))

(event Custom|SetHeatCurrent
  (params (Current :type Float%20%28single-precision%29))
  (Variables|Heat|SetHeatCurrent Current))

(event EventBeginPlay
  (CallFunction|Setup)
  (bind _ascore_gamemode_bp (Utilities|Casting|CastToCoreGamemodeBP (Game|GetGameMode)))
  (Default|AddTreeEntity (Variables|/Game/Blueprints/Gamemode/CoreGamemodeBP.CoreGamemodeBP_C|GetTreeManagerComponent _ascore_gamemode_bp) self))

(fn ConstructionScript)

(fn StopAllParticles
  (Effects|Particles|Trails|EndTrails (Variables|Default|GetFireSystem))
  (Effects|Particles|Trails|EndTrails (Variables|Default|GetSmokeSystem)))

(fn GetNearbyTrees
  (bind _self self)
  (bind _returnvalue (Transformation|GetActorLocation _self))
  (bind _outhits (Class|KismetSystemLibrary|CapsuleTraceMultiforObjects (+ _returnvalue "0, 0,-10.000000") (+ _returnvalue "0, 0,10.000000") 3.2e+02 2.0 (Utilities|Array|MakeArray "ObjectTypeQuery2") false 0 "None" true "(R=1.000000,G=0.000000,B=0.000000,A=1.000000)" "(R=0.000000,G=1.000000,B=0.000000,A=1.000000)" 3.0))
  (for _array_element _outhits
    (bind _astree_entity_actor_bp (Utilities|Casting|CastToTreeEntityActorBP (.HitActor (Collision|BreakHitResult _array_element))))
    (Utilities|Array|Add (Variables|Default|GetNearby) _astree_entity_actor_bp)))

(fn UpdateSmokeSystem
  (params (On :type Boolean))
  (bind _smokesystem (Variables|Default|GetSmokeSystem))
  (if On
    (Effects|Particles|Trails|BeginTrails _smokesystem "None" "None" "ETrailWidthMode_FromCentre" 0.0)
    (else
      (Effects|Particles|Trails|EndTrails _smokesystem))))

(fn UpdateFireSystem
  (params (On :type Boolean))
  (bind _firesystem (Variables|Default|GetFireSystem))
  (if On
    (Effects|Particles|Trails|BeginTrails _firesystem "None" "None" "ETrailWidthMode_FromCentre" 0.0)
    (else
      (Effects|Particles|Trails|EndTrails _firesystem))))

(fn SetBurnt
  (Components|StaticMesh|SetStaticMesh (Variables|Default|GetTree) "/Game/Assets/Nature/Trees/Tree_A_Burnt.Tree_A_Burnt")
  (Variables|Fire|SetisBurnt true))

(fn SetRegrown
  (Components|StaticMesh|SetStaticMesh (Variables|Default|GetTree) "/Game/Assets/Nature/Trees/Tree_A.Tree_A")
  (Variables|Fire|SetisBurnt false))