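; Seed actor that regrows nearby FireEntity actors when it is destroyed.
; On Destroyed, it runs a wide capsule multi-trace for WorldStatic objects around its Sphere component's location.
; Each hit actor that casts to FireEntity and is not currently on fire has Regrow called on it.
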(event EventBeginPlay)

(event Collision|EventActorBeginOverlap
  (params (OtherActor :type Actor%20Object%20Reference)))

(event EventTick
  (params (DeltaSeconds :type Float%20%28single-precision%29)))

(event EventDestroyed
  (bind _sphere (Variables|Default|GetSphere))
  (bind _returnvalue (Transformation|GetWorldLocation _sphere))
  (bind _outhits (Class|KismetSystemLibrary|CapsuleTraceMultiforObjects (+ _returnvalue "0, 0,-10.000000") (+ _returnvalue "0, 0,10.000000") 3e+02 2e+01 (Utilities|Array|MakeArray "ObjectTypeQuery1") false 0 "None" true))
  (for _array_element _outhits
    (bind _asfire_entity (Utilities|Casting|CastToFireEntity (.HitActor (Collision|BreakHitResult _array_element))))
    (if (not (Variables|/Game/Blueprints/Actors/Nature/Entities/FireEntity.FireEntity_C|GetisOnFire _asfire_entity))
      (Default|Regrow _asfire_entity))))

(fn ConstructionScript)