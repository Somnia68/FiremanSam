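; Water_PlaceHolder_BP is a placeholder water projectile that douses FireEntity actors.
; On spawn it scatters its launch velocity within a narrow cone at random speed and starts a timed self-destruct.
; Each overlap runs a small WorldStatic capsule trace, ignoring characters and tools gathered at spawn, and calls Water on the fire entities hit.
; The first successful hit shortens its lifespan to a fraction of a second.
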(event Custom|Kill
  (Actor|DestroyActor))

(event EventBeginPlay
  (bind _ignore (Variables|Default|GetIgnore))
  (|CallParentFunction)
  (Utilities|Time|SetTimerbyEvent (delegate Custom|Kill) 1e+01)
  (bind _outactors (Actor|GetAllActorsOfClass "/Game/Blueprints/Characters/Character_Base_BP.Character_Base_BP_C"))
  (Utilities|Array|AppendArray _ignore _outactors)
  (bind _outactors_2 (Actor|GetAllActorsOfClass "/Game/Blueprints/Actors/Tools/Tool_Base_BP.Tool_Base_BP_C"))
  (Utilities|Array|AppendArray _ignore _outactors_2)
  (Variables|/Script/Engine.MovementComponent|SetVelocity (Variables|Default|GetProjectileMovement) (* (Math|Random|RandomUnitVectorinConeinDegrees (Transformation|GetVelocity) 7.5) (Math|Random|RandomFloatinRange 5e+02 8e+02))))

(event Collision|EventActorBeginOverlap
  (params (OtherActor :type Actor%20Object%20Reference))
  (bind _staticmesh (Variables|Default|GetStaticMesh))
  (bind _returnvalue (Transformation|GetWorldLocation _staticmesh))
  (|CallParentFunction OtherActor)
  (bind _outhits (Class|KismetSystemLibrary|CapsuleTraceMultiforObjects (+ _returnvalue "0, 0,-10.000000") (+ _returnvalue "0, 0,10.000000") 6e+01 2e+01 (Utilities|Array|MakeArray "ObjectTypeQuery1") false (Variables|Default|GetIgnore) "None" true "(R=0.000000,G=0.808841,B=1.000000,A=1.000000)" "(R=0.000000,G=0.059623,B=1.000000,A=1.000000)" 0.016))
  (Variables|Default|SetHit false)
  (for _array_element _outhits
    (bind _asfire_entity (Utilities|Casting|CastToFireEntity (.HitActor (Collision|BreakHitResult _array_element))))
    (Default|Water _asfire_entity 12.0)
    (Variables|Default|SetHit true))
  (if (Variables|Default|GetHit)
    (if (not (Variables|Default|GetDying))
      (Actor|SetLifeSpan 0.2)
      (Variables|Default|SetDying true))))

(event EventTick
  (params (DeltaSeconds :type Float%20%28single-precision%29))
  (|CallParentFunction DeltaSeconds) ; This node is disabled and will not be called.\nDrag off pins to build functionality.
)

(fn ConstructionScript
  (|CallParentFunction))