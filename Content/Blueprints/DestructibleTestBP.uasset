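; DestructibleTestBP is a test Blueprint for inspecting hit events on a destructible component.
; Its custom event lajks matches the component hit signature and prints the hit component, other actor and component, normal impulse, a test string and the hit actor.
; The nodes that bind and unbind OnComponentHit are unconnected, so this graph never hooks up the event.
; BeginPlay, overlap and the construction script do nothing.
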(event Custom|lajks
  (params (HitComponent :type Primitive%20Component%20Object%20Reference) (OtherActor :type Actor%20Object%20Reference) (OtherComp :type Primitive%20Component%20Object%20Reference) (NormalImpulse :type Vector) (Hit :type Hit%20Result%20Structure%20%28by%20ref%29))
  (Development|PrintString (Utilities|GetDisplayName HitComponent))
  (Development|PrintString (Utilities|GetDisplayName OtherActor))
  (Development|PrintString (Utilities|GetDisplayName OtherComp))
  (Development|PrintString (Utilities|String|ToString(Vector) NormalImpulse))
  (Development|PrintString "Hello")
  (Development|PrintString (Utilities|GetDisplayName (.HitActor (Collision|BreakHitResult Hit)))))

(event EventBeginPlay)

(event Collision|EventActorBeginOverlap
  (params (OtherActor :type Actor%20Object%20Reference)))

(fn ConstructionScript)