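; SWFFGameMode is a game mode that publishes the world positions of up to two players to materials.
; BeginPlay disables tick, waits briefly, then re-enables it.
; Each tick, it writes the location of each valid pawn at player index 0 and 1 into the PlayerLocations material parameter collection as Player1 and Player2 vectors, packing XYZ into RGB.
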(event EventBeginPlay
  (Actor|Tick|SetActorTickEnabled false)
  (Utilities|FlowControl|Delay 2.0)
  (Actor|Tick|SetActorTickEnabled true))

(event EventTick
  (params (DeltaSeconds :type Float%20%28single-precision%29))
  (bind _returnvalue (Game|Player|GetPlayerPawn 1))
  (bind _returnvalue_2 (Game|Player|GetPlayerPawn 0))
  (bind _returnvalue_3 (Transformation|GetActorLocation _returnvalue))
  (bind _returnvalue_4 (Transformation|GetActorLocation _returnvalue_2))
  (bind (_x _y _z) (Math|Vector|BreakVector _returnvalue_3))
  (bind (_x_2 _y_2 _z_2) (Math|Vector|BreakVector _returnvalue_4))
  (Utilities|FlowControl|Sequence
    (:then_0
      (if (Utilities|IsValid _returnvalue_2)
        (Rendering|Material|SetVectorParameterValue "/Game/Materials/CommonUseMPC/PlayerLocations.PlayerLocations" "Player1" (Utilities|Struct|MakeLinearColor _x_2 _y_2 _z_2 0.0) :!class /Script/Engine.KismetMaterialLibrary)))
    (:then_1
      (if (Utilities|IsValid _returnvalue)
        (Rendering|Material|SetVectorParameterValue "/Game/Materials/CommonUseMPC/PlayerLocations.PlayerLocations" "Player2" (Utilities|Struct|MakeLinearColor _x _y _z 0.0) :!class /Script/Engine.KismetMaterialLibrary)))))

(fn ConstructionScript)