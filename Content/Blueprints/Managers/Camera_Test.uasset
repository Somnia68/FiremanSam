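; Shared two-player camera actor that keeps both Character_Base_BP players in view.
; After a short BeginPlay delay, PlayerSetup caches players 0 and 1 and makes itself every PlayerController's view target.
; Each tick, it moves to the players' midpoint and sets spring arm length from their separation, clamped between limits.
; The GameMode player list is stored but only read by an unconnected debug loop.
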(event EventBeginPlay
  (Actor|Tick|SetActorTickEnabled false)
  (Utilities|FlowControl|Delay 0.4)
  (CallFunction|PlayerSetup)
  (Actor|Tick|SetActorTickEnabled true))

(event EventTick
  (params (DeltaSeconds :type Float%20%28single-precision%29))
  (CallFunction|UpdateCamera))

(fn ConstructionScript)

(fn PlayerSetup
  (bind _ascharacter_base_bp (Utilities|Casting|CastToCharacter_Base_BP (Game|GetPlayerCharacter 0)))
  (Variables|Default|SetPlayer1 _ascharacter_base_bp)
  (bind _ascharacter_base_bp_2 (Utilities|Casting|CastToCharacter_Base_BP (Game|GetPlayerCharacter 1)))
  (Variables|Default|SetPlayer2 _ascharacter_base_bp_2)
  (bind _asfireman_sam_game_mode (Utilities|Casting|CastToFiremanSamGameMode (Game|GetGameMode)))
  (bind _output_get (Variables|Default|SetGameMode _asfireman_sam_game_mode))
  (Variables|Default|SetPlayersReference (Variables|/Game/Blueprints/Managers/FiremanSamGameMode.FiremanSamGameMode_C|GetPlayers _output_get))
  (bind _outactors (Actor|GetAllActorsOfClass "/Script/Engine.PlayerController"))
  (Game|Player|SetViewTargetwithBlend _outactors self 0.0 "VTBlend_Linear" 0.0 false))

(fn UpdateCamera
  (Variables|/Script/Engine.SpringArmComponent|SetTargetArmLength (Variables|Default|GetSpringArm) (Math|Float|Clamp(Float) (Transformation|GetDistanceTo (Variables|Default|GetPlayer1) (Variables|Default|GetPlayer2)) (Variables|Default|GetMinArmLength) (Variables|Default|GetMaxArmLength)))
  (Transformation|SetActorLocation (/ (+ (Transformation|GetActorLocation (Variables|Default|GetPlayer1)) (Transformation|GetActorLocation (Variables|Default|GetPlayer2))) 2.0) false false))