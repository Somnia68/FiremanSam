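; CameraManager is a shared camera actor that keeps two player characters framed from their midpoint.
; After a short BeginPlay delay, or on GameReady, it caches players 0 and 1 as CharacterBaseBP, sets itself as PlayerController view target and enables tick.
; Each tick moves the actor between both players and sets the spring arm length to their distance, clamped to minimum and maximum limits.
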(event Custom|GameReady
  (CallFunction|Setup)
  (Actor|Tick|SetActorTickEnabled true))

(event EventBeginPlay
  (Actor|Tick|SetActorTickEnabled false)
  (Utilities|FlowControl|Delay 0.2)
  (CallFunction|Setup)
  (Actor|Tick|SetActorTickEnabled true))

(event Collision|EventActorBeginOverlap
  (params (OtherActor :type Actor%20Object%20Reference)))

(event EventTick
  (params (DeltaSeconds :type Float%20%28single-precision%29))
  (CallFunction|UpdateCamera))

(fn ConstructionScript)

(fn Setup
  (bind _ascharacter_base_bp (Utilities|Casting|CastToCharacterBaseBP (Game|GetPlayerCharacter 0)))
  (Variables|Default|SetPlayer%201 _ascharacter_base_bp)
  (bind _ascharacter_base_bp_2 (Utilities|Casting|CastToCharacterBaseBP (Game|GetPlayerCharacter 1)))
  (Variables|Default|SetPlayer%202 _ascharacter_base_bp_2)
  (bind _outactors (Actor|GetAllActorsOfClass "/Script/Engine.PlayerController"))
  (Game|Player|SetViewTargetwithBlend _outactors self 0.0 "VTBlend_Linear" 0.0 false))

(fn UpdateCamera
  (Variables|/Script/Engine.SpringArmComponent|SetTargetArmLength (Variables|Default|GetSpringArm) (Math|Float|Clamp(Float) (Transformation|GetDistanceTo (Variables|Default|GetPlayer%201) (Variables|Default|GetPlayer%202)) (Variables|Default|GetMinArmLength) (Variables|Default|GetMaxArmLength)))
  (Transformation|SetActorLocation (/ (+ (Transformation|GetActorLocation (Variables|Default|GetPlayer%201)) (Transformation|GetActorLocation (Variables|Default|GetPlayer%202))) 2.0) false false))