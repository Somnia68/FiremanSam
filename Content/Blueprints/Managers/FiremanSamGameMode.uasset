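; Game mode for FiremanSam that spawns local players as Gardener or Firefighter characters when play begins.
; It gathers all PlayerStart actors, then matches each player index to the start whose tag equals that index.
; For each match it creates the player, spawns the character class selected by index, possesses it with that player's controller and records it in the Players array.
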(event EventBeginPlay
  (CallFunction|GetPlayerStartingPoints)
  (CallFunction|SpawnPlayers))

(event EventTick
  (params (DeltaSeconds :type Float%20%28single-precision%29)))

(fn ConstructionScript)

(fn GetPlayerStartingPoints
  (bind _outactors (Actor|GetAllActorsOfClass "/Script/Engine.PlayerStart"))
  (Variables|Default|SetPlayerStartArray _outactors))

(fn SpawnPlayers
  ;[1 1 1] Assigning Characters Dependent on what Character you are.
  (for _index (range 0 (- (Variables|Default|GetPlayerCount) 1))
    (Variables|Default|SetIndex _index)
    (for _array_element (Variables|Default|GetPlayerStartArray)
      (if (Utilities|Name|Equal(Name) (Variables|/Script/Engine.PlayerStart|GetPlayerStartTag _array_element) (Utilities|String|StringToName (Utilities|String|ToString(Integer) (Variables|Default|GetIndex))))
        (Class|GameplayStatics|CreatePlayer (Variables|Default|GetIndex))
        (bind _returnvalue (Game|SpawnActorfromClass (Utilities|Select :Index (Variables|Default|GetIndex) :Option%200 "/Game/Blueprints/Characters/Gardener_BP.Gardener_BP_C" :Option%201 "/Game/Blueprints/Characters/Firefighter_BP.Firefighter_BP_C") (Transformation|GetActorTransform _array_element) "AlwaysSpawn" 0 0))
        (bind _ascharacter_base_bp (Utilities|Casting|CastToCharacter_Base_BP _returnvalue))
        (Pawn|Possess (Game|GetPlayerController (Variables|Default|GetIndex)) _ascharacter_base_bp)
        (Utilities|Array|AddUnique (Variables|Default|GetPlayers) _ascharacter_base_bp)))))