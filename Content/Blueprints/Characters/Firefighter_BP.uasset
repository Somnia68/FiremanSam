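; Firefighter character Blueprint that sprays water while the FireCannon input is held.
; Pressing and releasing FireCannon opens and closes a Gate fed by Tick, so a Water_PlaceHolder_BP actor spawns every frame while held.
; Each water actor spawns slightly in front of the actor's location along the control rotation and takes that rotation, so the spray follows the aim.
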(event EventBeginPlay
  (|CallParentFunction))

(event Collision|EventActorBeginOverlap
  (params (OtherActor :type Actor%20Object%20Reference))
  (|CallParentFunction OtherActor) ; This node is disabled and will not be called.\nDrag off pins to build functionality.
)

(event EventTick
  (params (DeltaSeconds :type Float%20%28single-precision%29))
  (bind _returnvalue (Pawn|GetControlRotation :!class /Script/Engine.Pawn))
  (Utilities|FlowControl|Gate true
    (:Exit
      (Game|SpawnActorfromClass "/Game/Blueprints/Actors/Tools/Water_PlaceHolder_BP.Water_PlaceHolder_BP_C" (Math|Transform|MakeTransform (+ (Transformation|GetActorLocation) (* (Math|Vector|GetForwardVector _returnvalue) 1e+02)) _returnvalue) "Undefined" 0 0))))

(event Input|ActionEvents|InputActionFireCannon
  (params (Key :type Key%20Structure :default "None"))
  (bind _returnvalue (Pawn|GetControlRotation :!class /Script/Engine.Pawn))
  (:Pressed
    (Utilities|FlowControl|Gate true) ; enters at Open
  )
  (:Released
    (Utilities|FlowControl|Gate true) ; enters at Close
  ))

(fn ConstructionScript
  (|CallParentFunction))