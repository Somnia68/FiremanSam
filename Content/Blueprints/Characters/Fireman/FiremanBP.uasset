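; Fireman player character Blueprint that handles axis-driven movement and facing.
; MoveUp and MoveRight add movement input along world Y and X respectively, using the movement component's max speed as the direction component.
; LookUp and LookRight each set the actor's relative rotation from a single-axis vector, so each overwrites the other rather than combining into one aim direction.
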(event EventBeginPlay
  (|CallParentFunction) ; This node is disabled and will not be called.\nDrag off pins to build functionality.
)

(event Collision|EventActorBeginOverlap
  (params (OtherActor :type Actor%20Object%20Reference))
  (|CallParentFunction OtherActor) ; This node is disabled and will not be called.\nDrag off pins to build functionality.
)

(event EventTick
  (params (DeltaSeconds :type Float%20%28single-precision%29))
  (|CallParentFunction DeltaSeconds) ; This node is disabled and will not be called.\nDrag off pins to build functionality.
)

(event Input|AxisEvents|InputAxisMoveUp
  (params (AxisValue :type Float%20%28single-precision%29))
  (Pawn|Input|AddMovementInput (Math|Vector|MakeVector 0.0 (Class|MovementComponent|GetMaxSpeed (Variables|Character|GetCharacterMovement)) 0.0) AxisValue false))

(event Input|AxisEvents|InputAxisMoveRight
  (params (AxisValue :type Float%20%28single-precision%29))
  (Pawn|Input|AddMovementInput (Math|Vector|MakeVector (Class|MovementComponent|GetMaxSpeed (Variables|Character|GetCharacterMovement)) 0.0 0.0) AxisValue false))

(event Input|AxisEvents|InputAxisLookUp
  (params (AxisValue :type Float%20%28single-precision%29))
  (Transformation|SetActorRelativeRotation (Math|Conversions|RotationFromXVector (Math|Vector|MakeVector 0.0 AxisValue 0.0))))

(event Input|AxisEvents|InputAxisLookRight
  (params (AxisValue :type Float%20%28single-precision%29))
  (Transformation|SetActorRelativeRotation (Math|Conversions|RotationFromXVector (Math|Vector|MakeVector AxisValue 0.0 0.0))))

(fn ConstructionScript
  (|CallParentFunction))