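; Fireman character Blueprint that lets the player use firefighting tools.
; Input events forward tool switching, interaction, primary fire press and release, and a left-trigger analog axis to a FiremanToolComponent, which handles the tool behavior.
; The Blueprint adds no logic of its own; BeginPlay, overlap and Tick are disabled stubs, and the construction script only calls the parent.
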(event EventBeginPlay
  (|CallParentFunction) ; This node is disabled and will not be called.\nDrag off pins to build functionality.
)

(event Collision|EventActorBeginOverlap
  (params (OtherActor :type Actor%20Object%20Reference))
  (|CallParentFunction OtherActor) ; This node is disabled and will not be called.\nDrag off pins to build functionality.
)

(event EventTick
  (params (DeltaSeconds :type Float%20%28single-precision%29))
  (|CallParentFunction DeltaSeconds) ; This node is disabled and will not be called.\nDrag off pins to build functionality.
)

(event Input|ActionEvents|InputActionPrimaryAction
  (params (Key :type Key%20Structure :default "None"))
  (bind _firemantoolcomponent (Variables|Default|GetFiremanToolComponent))
  (:Pressed
    (Default|ToolFire _firemantoolcomponent))
  (:Released
    (Default|ToolStopFire _firemantoolcomponent)))

(event Input|ActionEvents|InputActionSwitchItem
  (params (Key :type Key%20Structure :default "None"))
  (:Pressed
    (Default|SwitchTools (Variables|Default|GetFiremanToolComponent))))

(event Input|ActionEvents|InputActionInteract
  (params (Key :type Key%20Structure :default "None"))
  (:Pressed
    (Default|ToolInteract (Variables|Default|GetFiremanToolComponent))))

(event Input|AxisEvents|InputAxisLeftTriggerAxis
  (params (AxisValue :type Float%20%28single-precision%29))
  (Default|ToolFireAxis (Variables|Default|GetFiremanToolComponent) AxisValue))

(fn ConstructionScript
  (|CallParentFunction))