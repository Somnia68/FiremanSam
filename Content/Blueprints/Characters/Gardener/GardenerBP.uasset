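; Gardener character Blueprint that turns player input into gardening and tool actions.
; Input events forward directly to GardenerToolComponent for planting seeds, healing trees, using the axe and dropping the pickup tank.
; Refilling opens on press and closes on release, while a separate axis event calls Refill without passing the axis value.
; BeginPlay and construction only call the parent, and Tick and overlap events are disabled.
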(event EventBeginPlay
  (|CallParentFunction))

(event Collision|EventActorBeginOverlap
  (params (OtherActor :type Actor%20Object%20Reference))
  (|CallParentFunction OtherActor) ; This node is disabled and will not be called.\nDrag off pins to build functionality.
)

(event EventTick
  (params (DeltaSeconds :type Float%20%28single-precision%29))
  (|CallParentFunction DeltaSeconds) ; This node is disabled and will not be called.\nDrag off pins to build functionality.
)

(event Input|ActionEvents|InputActionPrimaryUtilAction
  (params (Key :type Key%20Structure :default "None"))
  (:Pressed
    (Default|PlantSeed (Variables|Default|GetGardenerToolComponent))))

(event Input|ActionEvents|InputActionSecondaryUtilAction
  (params (Key :type Key%20Structure :default "None"))
  (:Pressed
    (Default|HealTree (Variables|Default|GetGardenerToolComponent))))

(event Input|ActionEvents|InputActionFireAction
  (params (Key :type Key%20Structure :default "None"))
  (:Pressed
    (Default|UseAxe (Variables|Default|GetGardenerToolComponent))))

(event Input|ActionEvents|InputActionGardenerDropTank
  (params (Key :type Key%20Structure :default "None"))
  (:Pressed
    (Default|Drop/PickupTank (Variables|Default|GetGardenerToolComponent))))

(event Input|ActionEvents|InputActionGardenerRefillAction
  (params (Key :type Key%20Structure :default "None"))
  (bind _gardenertoolcomponent (Variables|Default|GetGardenerToolComponent))
  (:Pressed
    (Default|OpenRefill _gardenertoolcomponent))
  (:Released
    (Default|CloseRefill _gardenertoolcomponent)))

(event Input|AxisEvents|InputAxisGardenerRefillAxis
  (params (AxisValue :type Float%20%28single-precision%29))
  (Default|Refill (Variables|Default|GetGardenerToolComponent)))

(fn ConstructionScript
  (|CallParentFunction))