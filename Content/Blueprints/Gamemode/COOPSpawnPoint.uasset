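; COOPSpawnPoint is a spawn point actor that sets up two-player local co-op with a Fireman and a Gardener.
; On BeginPlay it calls SpawnCOOP, which creates local players 0 and 1 in sequence.
; Each player's controller possesses a newly spawned FiremanBP or GardenerBP, respectively.
; Both pawns spawn at the actor's location plus their own offset variable, with zero rotation.
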(event Custom|SpawnCOOP
  (bind _returnvalue (Transformation|GetActorLocation))
  (Utilities|FlowControl|Sequence
    (:then_0
      (Class|GameplayStatics|CreatePlayer 0)
      (bind _returnvalue_2 (Game|SpawnActorfromClass "/Game/Blueprints/Characters/Fireman/FiremanBP.FiremanBP_C" (Math|Transform|MakeTransform (+ (Variables|Default|GetFiremanSpawn) _returnvalue)) "Undefined" 0 0))
      (Pawn|Possess (Game|GetPlayerController 0) _returnvalue_2))
    (:then_1
      (Class|GameplayStatics|CreatePlayer 1)
      (bind _returnvalue_3 (Game|SpawnActorfromClass "/Game/Blueprints/Characters/Gardener/GardenerBP.GardenerBP_C" (Math|Transform|MakeTransform (+ _returnvalue (Variables|Default|GetGardenerSpawn))) "Undefined" 0 0))
      (Pawn|Possess (Game|GetPlayerController 1) _returnvalue_3))))

(event EventBeginPlay
  (CallFunction|SpawnCOOP))

(event Collision|EventActorBeginOverlap
  (params (OtherActor :type Actor%20Object%20Reference)))

(event EventTick
  (params (DeltaSeconds :type Float%20%28single-precision%29)))

(fn ConstructionScript)